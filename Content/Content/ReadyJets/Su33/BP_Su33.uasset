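; Su-33 jet Blueprint that handles the startup sequence and cockpit screens of the flyable fighter.
; Activation timelines drive progress and body emissive, reveal displays and lights on remote instances, then set ReadyToFly; deactivation hides them again.
; Enabling the UI initializes the cockpit widgets and projects their render targets onto screen planes through dynamic materials, retrying until every target is valid.
; The afterburner event is empty, with its nozzle logic left disconnected.
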(event `self.ReceiveBeginPlay`
  ;[0.3931 1 0.2053] BeginPLay
  (`parent.ReceiveBeginPlay`)
  (`self.SetJetWidgetsVisibility` "Collapsed")
  (bind _asw_jet_mini_map (cast `/JETBORN/Content/ReadyJets/GenericJet_Content/UI/W_Jet_MiniMap` (`WidgetComponent.GetUserWidgetObject` (`self.MapDisplay`))))
  (`/JETBORN/Content/ReadyJets/GenericJet_Content/UI/W_Jet_MiniMap.InitializeMap` _asw_jet_mini_map self)
  (bind _asbpa_east_fighter_su_33 (cast `/JETBORN/Content/VigilanteContent/Vehicles/East_Fighter_Su33/BPA_East_Fighter_Su33` (`SkeletalMeshComponent.GetAnimInstance` (`self.VehicleMesh`))))
  (set `self.AnimInstance` _asbpa_east_fighter_su_33)
  (`self.SetAfterburner` false)
  (`SceneComponent.SetVisibility` (`self.AfterBurnerL`) true true)
  (`SceneComponent.SetVisibility` (`self.AfterBurnerR`) true true))

(event `ActivationSequence`
  ;[0 0 0] Set Ready to fly and materials
  (`|ExecutionSequence`
    (:`then_0`
      (set `self.ReadyToFly` false)
      (bind (_direction _progress) (`Timeline|Timeline_0` :!via `PlayFromStart`)
        (:`Update`
          (`SQHelicopterInstruments.SetActivationProgress` _progress)
          (`/Engine/EditorBlueprintResources/StandardMacros.DoOnce` false :!label _label
            (:`Completed`
              (`|ExecutionSequence`
                (:`then_0`
                  (`/Engine/EditorBlueprintResources/ActorMacros.Switch Has Authority`
                    (:`Remote`
                      (`KismetSystemLibrary.Delay` 4.0)
                      (`SceneComponent.SetVisibility` (`self.EngineStats`) true false)
                      (`SceneComponent.SetVisibility` (`self.PointLight_0`) true false)
                      (`SceneComponent.SetVisibility` (`self.PointLight1_0`) true false)
                      (`KismetSystemLibrary.Delay` 2.0)
                      (`SceneComponent.SetVisibility` (`self.MapDisplay`) true false)
                      (`SceneComponent.SetVisibility` (`self.DirectionScreen`) true false))))
                (:`then_1`
                  (bind (_direction_2 _lightintensity) (`Timeline|Timeline_1` :!label _label_2)
                    (:`Update`
                      (`MaterialInstanceDynamic.SetScalarParameterValue` (`self.BodyMaterial`) "EmissiveMult" _lightintensity))))))))
        (:`Finished`
          (set `self.ReadyToFly` true)
          (`LightComponent.SetLightColor` (`self.PointLight_0`) (struct :`G` 1.0 :`B` 0.635294 :`A` 1.0) true)
          (`LightComponent.SetLightColor` (`self.PointLight1_0`) (struct :`G` 1.0 :`B` 0.635294 :`A` 1.0) true))))
    (:`then_1`
      (goto _label_3 :!via `Reset`))))

(event `DeactivationSequence`
  ;[0 0 0] Set Ready to fly and materials
  (`/Engine/EditorBlueprintResources/StandardMacros.DoOnce` false :!label _label_3
    (:`Completed`
      (set `self.ReadyToFly` false)
      (`/Engine/EditorBlueprintResources/ActorMacros.Switch Has Authority`
        (:`Remote`
          (`LightComponent.SetLightColor` (`self.PointLight_0`) (struct :`R` 1.0 :`A` 1.0) true)
          (`LightComponent.SetLightColor` (`self.PointLight1_0`) (struct :`R` 1.0 :`A` 1.0) true)
          (`SceneComponent.SetVisibility` (`self.MapDisplay`) false false)
          (`SceneComponent.SetVisibility` (`self.DirectionScreen`) false false)
          (`SceneComponent.SetVisibility` (`self.EngineStats`) false false)
          (`SceneComponent.SetVisibility` (`self.PointLight_0`) false false)
          (`SceneComponent.SetVisibility` (`self.PointLight1_0`) false false)
          (`|ExecutionSequence`
            (:`then_0`
              (goto _label :!via `Reset`))
            (:`then_1`
              (goto _label_2 :!via `Stop`))))))))

(event `SetAfterburner`
  (params (Active :type Boolean)))

(event `self.Set UI Enabled`
  (params (`Enable UI` :type Boolean))
  (`/Engine/EditorBlueprintResources/StandardMacros.Can Execute Cosmetic Events`
    (:`True`
      (`self.ManageJetWidgets` `Enable UI`)
      (bind _all_valid_ (`self.SetJetWidgetMaterials` :!label _label_4))
      (if (not _all_valid_)
        (`KismetSystemLibrary.Delay` 0.4)
        (goto _label_4)))))

(fn `Get UI Tint`
  (returns (Color :type "LinearColor Structure"))
  (return (struct :`R` 0.505882 :`G` 1.0 :`B` 0.364706 :`A` 1.0)))

(fn `ManageJetWidgets`
  (params (Condition :type Boolean))
  (if Condition
    (`|ExecutionSequence`
      (:`then_0`
        (bind _asw_jet_main_display (cast `/JETBORN/Content/ReadyJets/GenericJet_Content/UI/W_JetMainDisplay` (`WidgetComponent.GetUserWidgetObject` (`self.MainDisplay`))))
        (`/JETBORN/Content/ReadyJets/GenericJet_Content/UI/W_JetMainDisplay.Set Owning Vehicle` _asw_jet_main_display self)
        (`/JETBORN/Content/ReadyJets/GenericJet_Content/UI/W_JetMainDisplay.Manage Update` _asw_jet_main_display true)
        (bind _asw_jet_compass_display (cast `/JETBORN/Content/ReadyJets/GenericJet_Content/UI/W_Jet_CompassDisplay` (`WidgetComponent.GetUserWidgetObject` (`self.Compass`))))
        (`/JETBORN/Content/ReadyJets/GenericJet_Content/UI/W_Jet_CompassDisplay.InitializeCompass` _asw_jet_compass_display self)
        (bind _asw_jet_engine_stats (cast `/JETBORN/Content/ReadyJets/GenericJet_Content/UI/W_Jet_EngineStats` (`WidgetComponent.GetUserWidgetObject` (`self.EngineStats`))))
        (`/JETBORN/Content/ReadyJets/GenericJet_Content/UI/W_Jet_EngineStats.InitializeDisplay` _asw_jet_engine_stats self (`self.Engine`) self)
        (bind _asw_jet_direction (cast `/JETBORN/Content/ReadyJets/GenericJet_Content/UI/W_JetDirection` (`WidgetComponent.GetUserWidgetObject` (`self.DirectionScreen`))))
        (`/JETBORN/Content/ReadyJets/GenericJet_Content/UI/W_JetDirection.InitializeScreen` _asw_jet_direction self))
      (:`then_1`
        (`self.SetJetWidgetsVisibility` "HitTestInvisible")))
    (else
      (`self.SetJetWidgetsVisibility` "Collapsed")
      (bind _asw_jet_main_display_2 (cast `/JETBORN/Content/ReadyJets/GenericJet_Content/UI/W_JetMainDisplay` (`WidgetComponent.GetUserWidgetObject` (`self.MainDisplay`))))
      (`/JETBORN/Content/ReadyJets/GenericJet_Content/UI/W_JetMainDisplay.Manage Update` _asw_jet_main_display_2 false))))

(fn `SetJetWidgetMaterials`
  (returns (`All Valid?` :type Boolean))
  (bind _screenmat (`self.ScreenMat`))
  (bind _returnvalue (`WidgetComponent.GetRenderTarget` (`self.MainDisplay`)))
  (bind _returnvalue_2 (`WidgetComponent.GetRenderTarget` (`self.Compass`)))
  (bind _returnvalue_3 (`WidgetComponent.GetRenderTarget` (`self.DirectionScreen`)))
  (bind _returnvalue_4 (`WidgetComponent.GetRenderTarget` (`self.EngineStats`)))
  (bind _returnvalue_5 (`WidgetComponent.GetRenderTarget` (`self.MapDisplay`)))
  (`SceneComponent.SetVisibility` (`self.MainDisplay`) true false)
  (`SceneComponent.SetVisibility` (`self.MapDisplay`) true false)
  (`SceneComponent.SetVisibility` (`self.Compass`) true false)
  (`SceneComponent.SetVisibility` (`self.EngineStats`) true false)
  (`SceneComponent.SetVisibility` (`self.DirectionScreen`) true false)
  (`WidgetComponent.RequestRenderUpdate` (`self.DirectionScreen`))
  (`WidgetComponent.RequestRenderUpdate` (`self.MainDisplay`))
  (`WidgetComponent.RequestRenderUpdate` (`self.MapDisplay`))
  (`WidgetComponent.RequestRenderUpdate` (`self.Compass`))
  (`WidgetComponent.RequestRenderUpdate` (`self.EngineStats`))
  ;[1 1 1] Project widgets to screen planes
  (bind _returnvalue_6 (`PrimitiveComponent.CreateDynamicMaterialInstance` (`self.Main Plane`) 0 _screenmat "None"))
  (`MaterialInstanceDynamic.SetTextureParameterValue` _returnvalue_6 "widgettexture" _returnvalue)
  (bind _returnvalue_7 (`PrimitiveComponent.CreateDynamicMaterialInstance` (`self.Compass Plane`) 0 _screenmat "None"))
  (`MaterialInstanceDynamic.SetTextureParameterValue` _returnvalue_7 "widgettexture" _returnvalue_2)
  (bind _returnvalue_8 (`PrimitiveComponent.CreateDynamicMaterialInstance` (`self.Map Plane`) 0 _screenmat "None"))
  (`MaterialInstanceDynamic.SetTextureParameterValue` _returnvalue_8 "widgettexture" _returnvalue_5)
  (bind _returnvalue_9 (`PrimitiveComponent.CreateDynamicMaterialInstance` (`self.Engine Stats Plane`) 0 _screenmat "None"))
  (`MaterialInstanceDynamic.SetTextureParameterValue` _returnvalue_9 "widgettexture" _returnvalue_4)
  (bind _returnvalue_10 (`PrimitiveComponent.CreateDynamicMaterialInstance` (`self.Direction Plane`) 0 _screenmat "None"))
  (`MaterialInstanceDynamic.SetTextureParameterValue` _returnvalue_10 "widgettexture" _returnvalue_3)
  (return (and (and (and (and (`KismetSystemLibrary.IsValid` _returnvalue) (`KismetSystemLibrary.IsValid` _returnvalue_2)) (`KismetSystemLibrary.IsValid` _returnvalue_5)) (`KismetSystemLibrary.IsValid` _returnvalue_4)) (`KismetSystemLibrary.IsValid` _returnvalue_3))))

(fn `SetJetWidgetsVisibility`
  (params (InVisibility :type "ESlateVisibility Enum" :default "Visible"))
  (`Widget.SetVisibility` (`WidgetComponent.GetUserWidgetObject` (`self.MainDisplay`)) InVisibility)
  (`Widget.SetVisibility` (`WidgetComponent.GetUserWidgetObject` (`self.Compass`)) InVisibility)
  (`Widget.SetVisibility` (`WidgetComponent.GetUserWidgetObject` (`self.EngineStats`)) InVisibility)
  (`Widget.SetVisibility` (`WidgetComponent.GetUserWidgetObject` (`self.DirectionScreen`)) InVisibility)
  (`Widget.SetVisibility` (`WidgetComponent.GetUserWidgetObject` (`self.MapDisplay`)) InVisibility))

(fn `UserConstructionScript`
  (`parent.UserConstructionScript`)
  (bind _returnvalue (`PrimitiveComponent.CreateDynamicMaterialInstance` (`self.VehicleMesh`) 0 "/JETBORN/Content/VigilanteContent/Vehicles/East_Fighter_Su33/Materials/MI_East_Fighter_Su33_Main.MI_East_Fighter_Su33_Main" "None"))
  (bind _output_get (set `self.BodyMaterial` _returnvalue))
  (`PrimitiveComponent.SetMaterial` (`self.VehicleMesh`) 0 _output_get)
  (`PrimitiveComponent.SetMaterial` (`self.VehicleMesh`) 0 _output_get)
  (bind _returnvalue_2 (`PrimitiveComponent.CreateDynamicMaterialInstance` (`self.VehicleMesh`) 0 "/JETBORN/Content/VigilanteContent/Vehicles/East_Fighter_Su33/Materials/MI_East_Fighter_Su33_Main.MI_East_Fighter_Su33_Main" "None"))
  (set `self.BodyMaterial` _returnvalue_2))